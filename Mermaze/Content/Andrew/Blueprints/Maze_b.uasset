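; Maze actor that, as written, builds the square outer wall of a tile grid, in both the construction script and BeginPlay.
; PopulateBorders appends the edge cells as flat indices to BorderTiles without clearing it.
; If ShowBorder is set, SpawnInstances converts indices via IntToGrid and adds scaled instances to the Wall instanced mesh.
; SetInitialTile seeds PathTiles with the first interior cell, but nothing calls it here.
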(event EventBeginPlay
  (CallFunction|PopulateBorders (Variables|Default|GetSize) (Variables|Default|GetBorder%20Tiles))
  (if (Variables|Default|GetShowBorder?)
    (Utilities|SpawnInstances (Variables|Default|GetBorder%20Tiles) (Variables|Default|GetSize) (Variables|Default|GetTileSize) "8.000000,8.000000,16.000000" (Variables|Default|GetWall))))

(fn ConstructionScript
  (CallFunction|PopulateBorders (Variables|Default|GetSize) (Variables|Default|GetBorder%20Tiles))
  (if (Variables|Default|GetShowBorder?)
    (Utilities|SpawnInstances (Variables|Default|GetBorder%20Tiles) (Variables|Default|GetSize) (Variables|Default|GetTileSize) "8.000000,8.000000,16.000000" (Variables|Default|GetWall))))

(fn PopulateBorders
  (params (Size :type Integer) (BorderArray :type Array%20of%20Integers))
  (LocalVariables|SetL_Size Size)
  (for _index (range 0 (- (LocalVariables|GetL_Size) 1))
    (Utilities|Array|Add BorderArray _index))
  (for _index_2 (range 1 (- (LocalVariables|GetL_Size) 2))
    (Utilities|Array|Add BorderArray (+ (* _index_2 (LocalVariables|GetL_Size)) (- (LocalVariables|GetL_Size) 1))))
  (for _index_3 (range 1 (LocalVariables|GetL_Size))
    (Utilities|Array|Add BorderArray (+ (- _index_3 1) (* (LocalVariables|GetL_Size) (- (LocalVariables|GetL_Size) 1)))))
  (for _index_4 (range 1 (- (LocalVariables|GetL_Size) 2))
    (Utilities|Array|Add BorderArray (* _index_4 (LocalVariables|GetL_Size)))))

(fn SetInitialTile
  (Variables|Default|SetCurrentTile (+ (Variables|Default|GetSize) 1))
  (Utilities|Array|Add (Variables|Default|GetPathTiles) (Variables|Default|GetCurrentTile)))