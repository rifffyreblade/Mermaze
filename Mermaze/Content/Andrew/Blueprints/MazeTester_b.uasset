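; Maze test Blueprint that lays out a rows-by-columns grid of Grid_Piece actors, each tagged with its grid coordinate.
; MakeMaze first builds row-letter and column-number name arrays, converting row counters to letters through an enum.
; It then spawns evenly spaced pieces, wrapping at each row's end and adding both names as separate actor tags.
; Afterwards it binds ReadyToSpawn to an event that only sets CanSpawn.
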(event `Make Maze`
  (bind _output_get (set `self.Total_Num` (* (`self.Rows-Num`) (`self.Columns_Num`))))
  (bind _returnvalue (- _output_get 1))
  (for _ (range (+ _returnvalue 1))
    (`self.BuildTags`))
  (for _index (range (+ _returnvalue 1))
    (`self.SpawnGrid` _index _index))
  (`KismetSystemLibrary.PrintString` "Done")
  (add `self.ReadyToSpawn` (delegate `Spawn`)))

(event `Spawn`
  (set `self.CanSpawn?` true))

(fn `UserConstructionScript`)