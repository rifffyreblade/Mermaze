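; Mermaid actor that moves its static mesh vertically with water levels and horizontally with the wind.
; BeginPlay caches four water heights around the start position; WaterRise compares current and target height, then steps the mesh with timelines, re-running through CheckWater until it matches the selected level.
; Swim and SwimBack share logic that plays or reverses a per-direction timeline based on CanMove, chaining another Swim after each forward finish.
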(event `self.ReceiveBeginPlay`
  (set `self.MyHeight` 3.0)
  (set `self.MinHeight` 3.0)
  (set `self.TargetHeight` 2.0)
  (bind _output_get (set `self.Origin` (`SceneComponent.K2_GetComponentLocation` (`self.StaticMeshComponent`))))
  (bind _x (.x _output_get))
  (bind _y (.y _output_get))
  (bind _z (.z _output_get))
  (set `self.Water_Level_0` (`KismetMathLibrary.MakeVector` _x _y (- _z 144.0)))
  (set `self.Water_Level_1` (`KismetMathLibrary.MakeVector` _x _y (- _z 72.0)))
  (set `self.Water_Level_2` (`KismetMathLibrary.MakeVector` _x _y _z))
  (set `self.Water_Level_3` (`KismetMathLibrary.MakeVector` _x _y (+ _z 72.0))))

(event `WaterRise`
  (bind _staticmeshcomponent (`self.StaticMeshComponent`))
  (bind _start (`self.Start`))
  (bind _start_2 (`self.Start`))
  (bind _returnvalue (+ (`self.MyHeight`) -1.0))
  (bind _returnvalue_2 (+ (`self.MyHeight`) 1.0))
  ;[0.3618 0.2094 1] Rise
  (bind _descend (`self.UpOrDown`)
    (:`End`
      (bind _output_get (set `self.Start` (`SceneComponent.K2_GetComponentLocation` (`self.StaticMeshComponent`))))
      (bind _dest (`self.WaterMove` (`self.Water_Level`) _output_get)
        (:`Move`
          (if _descend
            (if (> (`self.MyHeight`) (`self.MinHeight`))
              (if (not (== _start_2 (`self.Water_Level_0`)))
                (bind (_direction _rise) (`Timeline|Timeline_4` :!via `PlayFromStart`)
                  (:`Update`
                    (`SceneComponent.K2_SetWorldLocation` _staticmeshcomponent (`KismetMathLibrary.VLerp` _start_2 (`KismetMathLibrary.MakeVector` (.x _start_2) (.y _start_2) (+ (.z _start_2) (.z (0.0 0.0 -72.0)))) _rise) false false))
                  (:`Finished`
                    (if (not (< _returnvalue 0.0))
                      (set `self.MyHeight` _returnvalue)
                      (if (not (== (`SceneComponent.RelativeLocation` _staticmeshcomponent) _dest)) :!label _label
                        (`self.Check Water`)))))))
            (elif (not (== _start (`self.Water_Level_3`)))
              (bind (_direction_2 _rise_2) (`Timeline|Timeline_5` :!via `PlayFromStart`)
                (:`Update`
                  (`SceneComponent.K2_SetWorldLocation` _staticmeshcomponent (`KismetMathLibrary.VLerp` _start (`KismetMathLibrary.MakeVector` (.x _start) (.y _start) (+ (.z _start) (.z (0.0 0.0 72.0)))) _rise_2) false false))
                (:`Finished`
                  (if (not (> _returnvalue_2 3.0))
                    (set `self.MyHeight` _returnvalue_2)
                    (goto _label)))))))))))

(event `Swim Back`
  (bind _wind (`self.Wind`))
  (bind _staticmeshcomponent (`self.StaticMeshComponent`))
  (bind _start (`self.Start`))
  ;[1 1 1] Wind Mer Move
  (if (`self.Can Move?`) :!label _label_2
    (switch `/Game/Andrew/Blueprints/Wind_Direction` _wind
      (:`NewEnumerator0`
        (bind (_direction _rise) (`Timeline|Timeline_0` :!via `Reverse` :!label _label_3)
          (:`Update`
            (`SceneComponent.K2_SetWorldLocation` _staticmeshcomponent (`KismetMathLibrary.VLerp` _start (+ _start (0.0 100.0 0.0)) _rise) false false))
          (:`Finished`
            (if (select `ETimelineDirection` _direction :`Forward` true)
              (`self.Swim` :!label _label_4)
              (else
                (set `self.Can Move?` true :!label _label_5))))))
      (:`NewEnumerator1`
        (bind (_direction_2 _rise_2) (`Timeline|Timeline_1` :!via `Reverse` :!label _label_6)
          (:`Update`
            (`SceneComponent.K2_SetWorldLocation` _staticmeshcomponent (`KismetMathLibrary.VLerp` _start (+ _start (0.0 -100.0 0.0)) _rise_2) false false))
          (:`Finished`
            (if (select `ETimelineDirection` _direction_2 :`Forward` true)
              (goto _label_4)
              (else
                (goto _label_5))))))
      (:`NewEnumerator2`
        (bind (_direction_3 _rise_3) (`Timeline|Timeline_2` :!via `Reverse` :!label _label_7)
          (:`Update`
            (`SceneComponent.K2_SetWorldLocation` _staticmeshcomponent (`KismetMathLibrary.VLerp` _start (+ _start (-100.0 0.0 0.0)) _rise_3) false false))
          (:`Finished`
            (if (select `ETimelineDirection` _direction_3 :`Forward` true)
              (goto _label_4)
              (else
                (goto _label_5))))))
      (:`NewEnumerator3`
        (bind (_direction_4 _rise_4) (`Timeline|Timeline_3` :!via `Reverse` :!label _label_8)
          (:`Update`
            (`SceneComponent.K2_SetWorldLocation` _staticmeshcomponent (`KismetMathLibrary.VLerp` _start (+ _start (100.0 0.0 0.0)) _rise_4) false false))
          (:`Finished`
            (if (select `ETimelineDirection` _direction_4 :`Forward` true)
              (goto _label_4)
              (else
                (goto _label_5)))))))
    (else
      (set `self.Start` (`SceneComponent.K2_GetComponentLocation` (`self.StaticMeshComponent`)))
      (switch `/Game/Andrew/Blueprints/Wind_Direction` _wind
        (:`NewEnumerator0`
          (goto _label_3 :!via `PlayFromStart`))
        (:`NewEnumerator1`
          (goto _label_6 :!via `PlayFromStart`))
        (:`NewEnumerator2`
          (goto _label_7 :!via `PlayFromStart`))
        (:`NewEnumerator3`
          (goto _label_8 :!via `PlayFromStart`))))))

(event `Swim`
  ;[1 1 1] Wind Mer Move
  (goto _label_2))

(event `Check Water`
  ;[0.3618 0.2094 1] Rise
  (`self.WaterRise`))

(fn `UserConstructionScript`)