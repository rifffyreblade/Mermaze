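; Pirate actor that drifts with the wind and moves vertically with the water level.
; SwimBack and Swim step the mesh 100 units along the Wind direction through per-direction timelines, looping while CanMove holds.
; Overlapping an actor with Z scale above 3 reverses the current step and stops the drift.
; WaterRise, gated by CanDescend or Rising, lerps Z to one of four heights derived from the start position.
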(event `self.ReceiveBeginPlay`
  (bind _output_get (set `self.Origin` (`SceneComponent.K2_GetComponentLocation` (`self.StaticMeshComponent`))))
  (bind _x (.x _output_get))
  (bind _y (.y _output_get))
  (bind _z (.z _output_get))
  (set `self.Water_0` (`KismetMathLibrary.MakeVector` _x _y (- _z 72.0)))
  (set `self.Water_1` (`KismetMathLibrary.MakeVector` _x _y (- _z 0.0)))
  (set `self.Water_2` (`KismetMathLibrary.MakeVector` _x _y (+ _z 72.0)))
  (set `self.Water_3` (`KismetMathLibrary.MakeVector` _x _y (+ _z 144.0))))

(event `Swim Back`
  (bind _wind (`self.Wind`))
  (bind _staticmeshcomponent (`self.StaticMeshComponent`))
  (bind _start (`self.Start`))
  (if (`self.Can Move?`) :!label _label
    (set `self.Start` (`SceneComponent.K2_GetComponentLocation` (`self.StaticMeshComponent`)))
    (switch `/Game/Andrew/Blueprints/Wind_Direction` _wind
      (:`NewEnumerator0`
        (bind (_direction _rise) (`Timeline|Timeline_0` :!via `PlayFromStart` :!label _label_2)
          (:`Update`
            (`SceneComponent.K2_SetWorldLocation` _staticmeshcomponent (`KismetMathLibrary.VLerp` _start (+ _start (0.0 -100.0 0.0)) _rise) false false))
          (:`Finished`
            (if (select `ETimelineDirection` _direction :`Forward` true)
              (`self.Swim` :!label _label_3)
              (else
                (set `self.Can Move?` true :!label _label_4))))))
      (:`NewEnumerator1`
        (bind (_direction_2 _rise_2) (`Timeline|Timeline_1` :!via `PlayFromStart` :!label _label_5)
          (:`Update`
            (`SceneComponent.K2_SetWorldLocation` _staticmeshcomponent (`KismetMathLibrary.VLerp` _start (+ _start (0.0 100.0 0.0)) _rise_2) false false))
          (:`Finished`
            (if (select `ETimelineDirection` _direction_2 :`Forward` true)
              (goto _label_3)
              (else
                (goto _label_4))))))
      (:`NewEnumerator2`
        (bind (_direction_3 _rise_3) (`Timeline|Timeline_2` :!via `PlayFromStart` :!label _label_6)
          (:`Update`
            (`SceneComponent.K2_SetWorldLocation` _staticmeshcomponent (`KismetMathLibrary.VLerp` _start (+ _start (100.0 0.0 0.0)) _rise_3) false false))
          (:`Finished`
            (if (select `ETimelineDirection` _direction_3 :`Forward` true)
              (goto _label_3)
              (else
                (goto _label_4))))))
      (:`NewEnumerator3`
        (bind (_direction_4 _rise_4) (`Timeline|Timeline_3` :!via `PlayFromStart` :!label _label_7)
          (:`Update`
            (`SceneComponent.K2_SetWorldLocation` _staticmeshcomponent (`KismetMathLibrary.VLerp` _start (+ _start (-100.0 0.0 0.0)) _rise_4) false false))
          (:`Finished`
            (if (select `ETimelineDirection` _direction_4 :`Forward` true)
              (goto _label_3)
              (else
                (goto _label_4)))))))
    (else
      (switch `/Game/Andrew/Blueprints/Wind_Direction` _wind
        (:`NewEnumerator0`
          (goto _label_2 :!via `Reverse`))
        (:`NewEnumerator1`
          (goto _label_5 :!via `Reverse`))
        (:`NewEnumerator2`
          (goto _label_6 :!via `Reverse`))
        (:`NewEnumerator3`
          (goto _label_7 :!via `Reverse`))))))

(event `WaterRise`
  (bind _start (`self.Start`))
  (bind _start_2 (`self.Start`))
  (bind _start_3 (`self.Start`))
  (bind _start_4 (`self.Start`))
  ;[0.3618 0.2094 1] Rise
  (if (`self.Can Descend?`)
    (set `self.Start` (`SceneComponent.K2_GetComponentLocation` (`self.StaticMeshComponent`)) :!label _label_8)
    (switch `/Game/Chris/Water_Levels` (`self.Water_Level`)
      (:`NewEnumerator0`
        (bind (_direction _rise) (`Timeline|Timeline_4` :!via `PlayFromStart`)
          (:`Update`
            (`SceneComponent.K2_SetWorldLocation` (`self.StaticMeshComponent`) (`KismetMathLibrary.VLerp` _start_2 (`KismetMathLibrary.MakeVector` (.x _start_2) (.y _start_2) (.z (`self.Water_0`))) _rise) false false))))
      (:`NewEnumerator1`
        (bind (_direction_2 _rise_2) (`Timeline|Timeline_5` :!via `PlayFromStart`)
          (:`Update`
            (`SceneComponent.K2_SetWorldLocation` (`self.StaticMeshComponent`) (`KismetMathLibrary.VLerp` _start_3 (`KismetMathLibrary.MakeVector` (.x _start_3) (.y _start_3) (.z (`self.Water_1`))) _rise_2) false false))))
      (:`NewEnumerator2`
        (bind (_direction_3 _rise_3) (`Timeline|Timeline_6` :!via `PlayFromStart`)
          (:`Update`
            (`SceneComponent.K2_SetWorldLocation` (`self.StaticMeshComponent`) (`KismetMathLibrary.VLerp` _start_4 (`KismetMathLibrary.MakeVector` (.x _start_4) (.y _start_4) (.z (`self.Water_2`))) _rise_3) false false))))
      (:`NewEnumerator3`
        (bind (_direction_4 _rise_4) (`Timeline|Timeline_7` :!via `PlayFromStart`)
          (:`Update`
            (`SceneComponent.K2_SetWorldLocation` (`self.StaticMeshComponent`) (`KismetMathLibrary.VLerp` _start (`KismetMathLibrary.MakeVector` (.x _start) (.y _start) (.z (`self.Water_3`))) _rise_4) false false)))))
    (elif (`self.Rising?`)
      (goto _label_8))))

(event `Swim`
  (goto _label))

(event `self.ReceiveActorBeginOverlap`
  (params (OtherActor :type "Actor Object Reference"))
  (if (> (.z (`self.GetActorScale3D` OtherActor)) 3.0)
    (set `self.Can Move?` false)
    (`self.Swim Back`)))

(event `self.ReceiveActorEndOverlap`
  (params (OtherActor :type "Actor Object Reference"))
  (set `self.Old Sea Level` 0.0))

(fn `UserConstructionScript`)