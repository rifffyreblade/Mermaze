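; Maze blueprint that builds a grid of height-scaled instanced static mesh tiles at BeginPlay.
; SetVector feeds tile coordinates and seeded random heights into TilesArray, then OverrideZ forces a tall border and fixed heights at two inner corners.
; BuildMe adds each instance, prints its letter-number grid tag and stores a capsule transform before calling CallMakeCollide.
; Hit events print the other object's name.
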(event `self.ReceiveBeginPlay`
  (`self.BuildMe`))

(event `self.ReceiveHit`
  (params (MyComp :type "PrimitiveComponent Object Reference") (Other :type "Actor Object Reference") (OtherComp :type "PrimitiveComponent Object Reference") (bSelfMoved :type Boolean) (HitLocation :type "Vector Structure") (HitNormal :type "Vector Structure") (NormalImpulse :type "Vector Structure") (Hit :type "HitResult Structure (by ref)"))
  (`KismetSystemLibrary.PrintString` (`KismetSystemLibrary.GetDisplayName` Other)))

(fn `BuildMe`
  (bind _index (`self.Index`))
  (bind _tilesarray (`self.TilesArray`))
  (bind _nextvec (`self.SetVector`)
    (:`Out`
      (bind _returnvalue (`KismetArrayLibrary.Array_Add` _tilesarray _nextvec))
      (if (== _returnvalue 0)
        (bind _output_get (set `self.LastVec` (`KismetArrayLibrary.Array_Get` _tilesarray (- (stale _index_2) 1)))))
      (for _index_2 (range _index (+ (`KismetArrayLibrary.Array_LastIndex` _tilesarray) 1))
        (bind _item (`KismetArrayLibrary.Array_Get` _tilesarray _index_2))
        (bind _new_z (`self.OverrideZ` (.x _item) (.y _item) (.z _item))
          (:`Out`
            (set `self.Index` (+ _index 1))
            (bind _returnvalue_2 (`KismetMathLibrary.MakeVector` 1.0 1.0 _new_z))
            (bind _returnvalue_3 (`KismetMathLibrary.MakeTransform` (* (+ _output_get _item) (100.0 100.0 0.0)) (struct) (* _returnvalue_2 (1.0 1.0 0.5))))
            (`InstancedStaticMeshComponent.AddInstance` (`self.InstancedStaticMesh`) _returnvalue_3)
            (if (>= (`self.ColumnInt`) 9)
              (set `self.Row_Int` (+ (`self.Row_Int`) 1))
              (set `self.ColumnInt` 0))
            (bind _tag (`self.Set Tag` (`self.Row_Int`) (`self.ColumnInt`))
              (:`Out`
                (set `self.ColumnInt` (+ (`self.ColumnInt`) 1))
                (`KismetSystemLibrary.PrintString` _tag)
                (bind _location (.location _returnvalue_3))
                (set `self.Capsule_Trans` (`KismetMathLibrary.MakeTransform` (`KismetMathLibrary.MakeVector` (.x _location) (.y _location) 50.0) (struct) (* _returnvalue_2 (1.0 1.0 1.0))))
                (set `self.Capsule Loc` _location)
                (`self.MakeCollide`)))))))))

(fn `UserConstructionScript`)