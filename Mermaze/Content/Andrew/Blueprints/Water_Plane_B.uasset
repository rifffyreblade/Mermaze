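; Water plane actor that moves its mesh vertically between four preset water levels.
; BeginPlay triggers WaterRise, then derives the level positions from the mesh's starting location in evenly spaced upward steps.
; WaterRise switches on the WaterLevel enum, stores the current position through SetPosition, and plays that level's own timeline to lerp the mesh from there to the target.
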(event `self.ReceiveBeginPlay`
  ;[1 1 1] Sets Variables
  (`self.WaterRise`)
  (bind _output_get (set `self.Water_Level_0` (`SceneComponent.K2_GetComponentLocation` (`self.StaticMeshComponent`))))
  (bind _output_get_2 (set `self.Water_Level_1` (+ _output_get (0.0 0.0 48.0))))
  (bind _output_get_3 (set `self.Water_Level_2` (+ _output_get_2 (0.0 0.0 48.0))))
  (set `self.Water_Level_3` (+ _output_get_3 (0.0 0.0 48.0))))

(event `WaterRise`
  ;[0.3618 0.2094 1] Rise
  (switch `/Game/Andrew/Blueprints/Water_Levels` (`self.Water_Level`)
    (:`NewEnumerator0`
      (`self.Set Position`)
      (bind (_direction _rise) (`Timeline|Level_0 Time` :!via `PlayFromStart`)
        (:`Update`
          (`SceneComponent.K2_SetWorldLocation` (`self.StaticMeshComponent`) (`KismetMathLibrary.VLerp` (`self.Start`) (`self.Water_Level_0`) _rise) false false))))
    (:`NewEnumerator1`
      (`self.Set Position`)
      (bind (_direction_2 _rise_2) (`Timeline|Timeline_0` :!via `PlayFromStart`)
        (:`Update`
          (`SceneComponent.K2_SetWorldLocation` (`self.StaticMeshComponent`) (`KismetMathLibrary.VLerp` (`self.Start`) (`self.Water_Level_1`) _rise_2) false false))))
    (:`NewEnumerator2`
      (`self.Set Position`)
      (bind (_direction_3 _rise_3) (`Timeline|Timeline_1` :!via `PlayFromStart`)
        (:`Update`
          (`SceneComponent.K2_SetWorldLocation` (`self.StaticMeshComponent`) (`KismetMathLibrary.VLerp` (`self.Start`) (`self.Water_Level_2`) _rise_3) false false))))
    (:`NewEnumerator3`
      (`self.Set Position`)
      (bind (_direction_4 _rise_4) (`Timeline|Timeline_2` :!via `PlayFromStart`)
        (:`Update`
          (`SceneComponent.K2_SetWorldLocation` (`self.StaticMeshComponent`) (`KismetMathLibrary.VLerp` (`self.Start`) (`self.Water_Level_3`) _rise_4) false false))))))

(fn `Set Position`
  (set `self.Start` (`SceneComponent.K2_GetComponentLocation` (`self.StaticMeshComponent`))))

(fn `UserConstructionScript`)